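; BP_FloorTile is a self-replacing floor segment for an endless runner that spawns either a damage box or coins.
; Its construction script randomly places one box at the right, middle or left spawn point, or scatters coins inside CoinArea, as child actors.
; When a SideScrollerCharacter first overlaps EndTrigger, it asks LevelGameMode to add a tile, then destroys itself after a short delay.
; GetAttachTransform exposes AttachPoint's world transform.
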(event `self.EndTrigger.OnComponentBeginOverlap`
  (params (OverlappedComponent :type "PrimitiveComponent Object Reference") (OtherActor :type "Actor Object Reference") (OtherComp :type "PrimitiveComponent Object Reference") (OtherBodyIndex :type Integer) (bFromSweep :type Boolean) (SweepResult :type "HitResult Structure (by ref)"))
  (cast `/Game/GloryRunProject/Blueprints/Character/SideScrollerCharacter` OtherActor)
  (`/Engine/EditorBlueprintResources/StandardMacros.DoOnce` false
    (:`Completed`
      (bind _aslevel_game_mode (cast `/Game/GloryRunProject/Blueprints/Modes/LevelGameMode` (`GameplayStatics.GetGameMode`)))
      (`/Game/GloryRunProject/Blueprints/Modes/LevelGameMode.AddFloorTile` _aslevel_game_mode)
      (`KismetSystemLibrary.Delay` 2.0)
      (`self.K2_DestroyActor`))))

(fn `GetAttachTransform`
  (returns (AttachTransform :type "Transform Structure"))
  (return (`SceneComponent.K2_GetComponentToWorld` (`self.AttachPoint`))))

(fn `SetSpawnPoints`
  (set `self.SpawnPoint` (`|MakeArray` (`SceneComponent.GetRelativeTransform` (`self.SpawnPointRight`)) (`SceneComponent.GetRelativeTransform` (`self.SpawnPointMid`)) (`SceneComponent.GetRelativeTransform` (`self.SpawnPointLeft`)))))

(fn `SpawnCoins`
  (bind _coinarea (`self.CoinArea`))
  (for _ (range 6)
    (`AddComponent|NODE_AddChildActorComponent-1` :`RelativeTransform` (`KismetMathLibrary.Conv_VectorToTransform` (`KismetMathLibrary.RandomPointInBoundingBox` (`SceneComponent.RelativeLocation` _coinarea) (`BoxComponent.BoxExtent` _coinarea))))))

(fn `SpawnDamageBox`
  (bind _spawnpoint (`self.SpawnPoint`))
  (`AddComponent|NODE_AddChildActorComponent-0` :`RelativeTransform` (`|GetArrayItem` _spawnpoint (`KismetMathLibrary.RandomIntegerInRange` 0 (`KismetArrayLibrary.Array_LastIndex` _spawnpoint)))))

(fn `UserConstructionScript`
  (`self.SetSpawnPoints`)
  (switch `int` (`KismetMathLibrary.RandomIntegerInRange` 0 1)
    (:`Default`
      (`self.SpawnDamageBox` :!label _label))
    (:`0`
      (goto _label))
    (:`1`
      (`self.SpawnCoins`))))